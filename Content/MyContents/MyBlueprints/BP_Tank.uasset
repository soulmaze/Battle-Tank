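; BP_Tank is a player-controllable tank with orbit-style aiming and a fire action.
; On BeginPlay it passes its barrel and turret components to setter functions defined outside these graphs.
; Aim axes rotate an azimuth gimbal for yaw and the spring arm for pitch, scaled by frame time, keeping the two rotations on separate components.
; Pressing Fire calls a Fire function, also defined elsewhere.
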(event `self.ReceiveBeginPlay`
  (`self.SetBarrelRefrence` (`self.TankBarrel1`))
  (`self.SetTurretRefrence` (`self.TankTurret`)))

(event `InputAxis|AimAzimuth`
  (params (AxisValue :type "Float (single-precision)"))
  ;[1 1 1] Input Bindings
  (`SceneComponent.K2_AddLocalRotation` (`self.AzimuthGimbal`) (`KismetMathLibrary.MakeRotator` 0.0 0.0 (* AxisValue (`GameplayStatics.GetWorldDeltaSeconds`) 100.0)) false false))

(event `InputAxis|AimElevation`
  (params (AxisValue :type "Float (single-precision)"))
  ;[1 1 1] Input Bindings
  (`SceneComponent.K2_AddLocalRotation` (`self.SpringArm`) (`KismetMathLibrary.MakeRotator` 0.0 (* AxisValue (`GameplayStatics.GetWorldDeltaSeconds`) 100.0)) false false))

(event `InputAction|Fire`
  (params (Key :type "Key Structure"))
  ;[1 1 1] Input Bindings
  (:`Pressed`
    (`self.Fire`)))

(fn `UserConstructionScript`)